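; BP_Console is an interactable console that presents one of several games, or the credits, chosen by GameToPresent.
; On BeginPlay it sets the matching hologram material and preview widget logo; Credits instead swaps in a credits widget and hides the hologram plane and Niagara effect.
; Interact adds a WBP_Console to the viewport, hands it a reference to this console and reveals the section for that selection.
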(event EventBeginPlay
  (Rendering|Material|SetMaterial (Variables|Default|GetPlane_Hologram) 0 (Utilities|Select :Index (Variables|Default|GetGameToPresent) :NewEnumerator0 "/Game/Assets/UI_Assets/M_Hologram_SAA.M_Hologram_SAA" :NewEnumerator1 "/Game/Assets/UI_Assets/M_Hologram_FB.M_Hologram_FB" :NewEnumerator2 "/Game/Assets/UI_Assets/M_Hologram_WFA.M_Hologram_WFA" :NewEnumerator3 0))
  (bind _aswbp_console_preview (Utilities|Casting|CastToWBP_ConsolePreview (UserInterface|GetWidget (Variables|Default|GetWidget))))
  (switch Utilities|FlowControl|Switch|SwitchonE_Games (Variables|Default|GetGameToPresent)
    (:NewEnumerator0
      (Appearance|SetBrushfromTexture (Variables|/Game/Blueprints/ThisProject/WBP_ConsolePreview.WBP_ConsolePreview_C|GetImage_Logo _aswbp_console_preview) "/Game/Assets/UI_Assets/Images/SAA_Logo_Retouched.SAA_Logo_Retouched" false))
    (:NewEnumerator1
      (Appearance|SetBrushfromTexture (Variables|/Game/Blueprints/ThisProject/WBP_ConsolePreview.WBP_ConsolePreview_C|GetImage_Logo _aswbp_console_preview) "/Game/Assets/UI_Assets/Images/FB_Logo_Retouched.FB_Logo_Retouched" false))
    (:NewEnumerator2
      (Appearance|SetBrushfromTexture (Variables|/Game/Blueprints/ThisProject/WBP_ConsolePreview.WBP_ConsolePreview_C|GetImage_Logo _aswbp_console_preview) "/Game/Assets/UI_Assets/Images/WFA_Logo_Retouched.WFA_Logo_Retouched" false))
    (:NewEnumerator3
      (bind _returnvalue (UserInterface|CreateWidget "/Game/Blueprints/ThisProject/WBP_Credits.WBP_Credits_C"))
      (UserInterface|SetWidget (Variables|Default|GetWidget) _returnvalue)
      (Rendering|SetVisibility (Variables|Default|GetPlane_Hologram) false false)
      (Rendering|SetVisibility (Variables|Default|GetNiagara) false false))))

(event EventInteract
  (bind _returnvalue (UserInterface|CreateWidget "/Game/Blueprints/ThisProject/WBP_Console.WBP_Console_C"))
  (Variables|/Game/Blueprints/ThisProject/WBP_Console.WBP_Console_C|SetConsoleRef _returnvalue self)
  (UserInterface|Viewport|AddtoViewport _returnvalue 0)
  (switch Utilities|FlowControl|Switch|SwitchonE_Games (Variables|Default|GetGameToPresent)
    (:NewEnumerator0
      (Widget|SetVisibility (Variables|/Game/Blueprints/ThisProject/WBP_Console.WBP_Console_C|GetGrid_SAA _returnvalue) "SelfHitTestInvisible"))
    (:NewEnumerator1
      (Widget|SetVisibility (Variables|/Game/Blueprints/ThisProject/WBP_Console.WBP_Console_C|GetGrid_FB _returnvalue) "SelfHitTestInvisible"))
    (:NewEnumerator2
      (Widget|SetVisibility (Variables|/Game/Blueprints/ThisProject/WBP_Console.WBP_Console_C|GetGrid_WFA _returnvalue) "SelfHitTestInvisible"))
    (:NewEnumerator3
      (Widget|SetVisibility (Variables|/Game/Blueprints/ThisProject/WBP_Console.WBP_Console_C|GetWBP_Credits _returnvalue) "SelfHitTestInvisible"))))

(fn ConstructionScript)