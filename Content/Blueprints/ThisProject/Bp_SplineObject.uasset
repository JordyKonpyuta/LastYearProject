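; Spline path actor that spawns a ship and moves it along the spline over a set time.
; On BeginPlay it spawns the ShipToSpawn class at the Arrow component's transform and stores it as Ship.
; A timeline, play rate scaled by TimeToComplete, lerps distance along the spline each update.
; The ship takes that point's world location and rotation, with yaw offset by 90 degrees.
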(event Custom|MoveObject
  (bind _spline (Variables|Default|GetSpline))
  (Components|Timeline|SetPlayRate (Variables|Default|GetT_Move) (/ 1.0 (Variables|Default|GetTimeToComplete)))
  (bind _newtrack_0 (Timeline|T_Move Play)
    (:Update
      (Transformation|SetActorLocationAndRotation (Variables|Default|GetShip) (Spline|GetLocationatDistanceAlongSpline _spline (Math|Float|Lerp 0.0 (Spline|GetSplineLength _spline) _newtrack_0) "World") (Math|Rotator|MakeRotator (.roll (Spline|GetRotationatDistanceAlongSpline _spline (Math|Float|Lerp 0.0 (Spline|GetSplineLength _spline) _newtrack_0) "World")) (.pitch (Spline|GetRotationatDistanceAlongSpline _spline (Math|Float|Lerp 0.0 (Spline|GetSplineLength _spline) _newtrack_0) "World")) (- (.yaw (Spline|GetRotationatDistanceAlongSpline _spline (Math|Float|Lerp 0.0 (Spline|GetSplineLength _spline) _newtrack_0) "World")) 9e+01))))))

(event EventBeginPlay
  (bind _returnvalue (Game|SpawnActorfromClass (Variables|Default|GetShipToSpawn) (Transformation|GetWorldTransform (Variables|Default|GetArrow)) "AdjustIfPossibleButAlwaysSpawn" "MultiplyWithRoot" 0 0))
  (Variables|Default|SetShip _returnvalue)
  (CallFunction|MoveObject))

(fn ConstructionScript)