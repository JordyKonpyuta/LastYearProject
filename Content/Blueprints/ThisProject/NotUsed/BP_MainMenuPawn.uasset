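; Main menu pawn that shows the mouse cursor, sets Game and UI input on BeginPlay, and provides smooth camera moves.
; CameraMovement stores a target location and rotation, then starts a fast looping timer, presumably bound to MoveCamera.
; MoveCamera eases the camera toward both targets with VInterpTo and RInterpTo using world delta time.
; The timer clears only on an exact location match; rotation is not checked.
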(event Custom|MoveCamera
  (bind _returnvalue (Utilities|Time|GetWorldDeltaSeconds))
  (bind _camera (Variables|Default|GetCamera))
  (bind _returnvalue_2 (Transformation|GetWorldLocation _camera))
  (Transformation|SetWorldLocationAndRotation _camera (Math|Interpolation|VInterpTo _returnvalue_2 (Variables|Default|GetTargetLocation) _returnvalue 0.5) (Math|Interpolation|RInterpTo (Transformation|GetWorldRotation _camera) (Variables|Default|GetTargetRotation) _returnvalue 0.5) false false)
  (if (Utilities|Operators|EqualEqual _returnvalue_2 (Variables|Default|GetTargetLocation) 0.0)
    (Utilities|Time|ClearandInvalidateTimerbyHandle (Variables|Default|GetTimerHandle))))

(event Custom|CameraMovement
  (params (TargetLocation :type Vector) (TargetRotation :type Rotator))
  (Variables|Default|SetTargetLocation TargetLocation)
  (Variables|Default|SetTargetRotation TargetRotation)
  (bind _returnvalue (Utilities|Time|SetTimerbyEvent (EventDispatchers|CreateEvent :!event Custom|MoveCamera) 0.001 true))
  (Variables|Default|SetTimerHandle _returnvalue))

(event EventBeginPlay
  (bind _returnvalue (Game|GetPlayerController 0))
  (Variables|/Script/Engine.PlayerController|SetbShowMouseCursor _returnvalue true)
  (Input|SetInputModeGameandUI _returnvalue 0 "DoNotLock" true true))

(fn ConstructionScript)