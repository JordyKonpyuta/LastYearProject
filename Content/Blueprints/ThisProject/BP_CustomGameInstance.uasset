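; Game instance that holds persistent player progress: money, owned furniture, win/loss record and tournament unlocks.
; It creates, loads and writes a BP_SaveGameSystem slot for new game and continue.
; Finishing a tournament pays money by difficulty and win count, records victory or defeat, unlocks the next tier and saves.
; InitTournament filters the trainer data table by difficulty and randomly trims it to at most three opponents.
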(event Custom|NewGame
  (bind _returnvalue (SaveGame|DoesSaveGameExist (Variables|FurnitureBattle|GetSaveName)))
  (if _returnvalue
    (SaveGame|DeleteGameinSlot (Variables|FurnitureBattle|GetSaveName)))
  (CallFunction|CreateSaveData)
  (Utilities|FlowControl|Delay 0.5)
  (Game|OpenLevel(byName) "None"))

(event Custom|SaveGame
  (bind _sauvegarde (Variables|FurnitureBattle|GetSauvegarde))
  ;[0.1314 0.9203 1 0.5 48] Sauvegarde
  (Variables|/Game/Blueprints/FB/BP_SaveGameSystem.BP_SaveGameSystem_C|SetArgent _sauvegarde (Variables|FurnitureBattle|GetArgentActuel))
  (Variables|/Game/Blueprints/FB/BP_SaveGameSystem.BP_SaveGameSystem_C|SetMeublesDeverouilles _sauvegarde (Variables|FurnitureBattle|GetMeublesPossedes))
  (Variables|/Game/Blueprints/FB/BP_SaveGameSystem.BP_SaveGameSystem_C|SetVictoires _sauvegarde (Variables|FurnitureBattle|GetVictoires))
  (Variables|/Game/Blueprints/FB/BP_SaveGameSystem.BP_SaveGameSystem_C|SetDefaites _sauvegarde (Variables|FurnitureBattle|GetDefaites))
  (SaveGame|SaveGametoSlot _sauvegarde (Variables|FurnitureBattle|GetSaveName)))

(event Custom|LoadGame
  ;[1 0.7309 0 0.5 48] Load Save Data
  (bind _returnvalue (SaveGame|LoadGamefromSlot (Variables|FurnitureBattle|GetSaveName)))
  (bind _asbp_save_game_system (Utilities|Casting|CastToBP_SaveGameSystem _returnvalue))
  (bind _output_get (Variables|FurnitureBattle|SetSauvegarde _asbp_save_game_system))
  (Variables|FurnitureBattle|SetArgentActuel (Variables|/Game/Blueprints/FB/BP_SaveGameSystem.BP_SaveGameSystem_C|GetArgent _output_get))
  (Variables|FurnitureBattle|SetMeublesPossedes (Variables|/Game/Blueprints/FB/BP_SaveGameSystem.BP_SaveGameSystem_C|GetMeublesDeverouilles _output_get))
  (Variables|FurnitureBattle|SetVictoires (Variables|/Game/Blueprints/FB/BP_SaveGameSystem.BP_SaveGameSystem_C|GetVictoires _output_get))
  (Variables|FurnitureBattle|SetDefaites (Variables|/Game/Blueprints/FB/BP_SaveGameSystem.BP_SaveGameSystem_C|GetDefaites _output_get))
  (Variables|FurnitureBattle|SetTournoi2Debloque (Variables|/Game/Blueprints/FB/BP_SaveGameSystem.BP_SaveGameSystem_C|GetTournoi2Debloque _output_get))
  (Variables|FurnitureBattle|SetTournoi3Debloque (Variables|/Game/Blueprints/FB/BP_SaveGameSystem.BP_SaveGameSystem_C|GetTournoi3Debloque _output_get)))

(event Custom|Create%20Save%20Data
  ;[0.01548 0.15 0 0.5 36] Create Save Data
  (bind _returnvalue (SaveGame|CreateSaveGameObject "/Game/Blueprints/FB/BP_SaveGameSystem.BP_SaveGameSystem_C"))
  (SaveGame|SaveGametoSlot _returnvalue (Variables|FurnitureBattle|GetSaveName))
  (Variables|FurnitureBattle|SetSauvegarde _returnvalue)
  (CallFunction|SaveGame))

(event Custom|TournoiTermine
  (params (NombreDeVictoires :type Integer))
  ;[0.6198 0.1355 0.4813 0.5 36] Completer un Tournoi
  (Variables|FurnitureBattle|SetGainArgent (Math|Float|Truncate (* (Utilities|Select :Index (Variables|FurnitureBattle|GetTournoiDifficulte) :NewEnumerator0 200 :NewEnumerator1 300 :NewEnumerator2 400) (Utilities|Select :Index NombreDeVictoires :Option%200 0.25 :Option%201 0.5 :Option%202 0.75 :Option%203 1.0))))
  (if (>= NombreDeVictoires 3)
    (Math|Integer|IncrementInt (Variables|FurnitureBattle|GetVictoires)
      (:%20%20
        (switch Utilities|FlowControl|Switch|SwitchonEnum_TournamentClass (Variables|FurnitureBattle|GetTournoiDifficulte)
          (:NewEnumerator0
            (Variables|FurnitureBattle|SetTournoi2Debloque true))
          (:NewEnumerator1
            (Variables|FurnitureBattle|SetTournoi3Debloque true))
          (:NewEnumerator2
            _))))
    (else
      (Math|Integer|IncrementInt (Variables|FurnitureBattle|GetDefaites)
        (:%20%20
          _))))
  (CallFunction|SauvegardeTournois)
  (Variables|FurnitureBattle|SetArgentActuel (+ (Variables|FurnitureBattle|GetArgentActuel) (Variables|FurnitureBattle|GetGainArgent)))
  (CallFunction|SaveGame))

(event Custom|SauvegardeTournois
  (bind _sauvegarde (Variables|FurnitureBattle|GetSauvegarde))
  ;[0 0.1703 1 0.5 30] Sauvegarde Spécifique - Tournois
  (Variables|/Game/Blueprints/FB/BP_SaveGameSystem.BP_SaveGameSystem_C|SetTournoi2Debloque _sauvegarde (Variables|FurnitureBattle|GetTournoi2Debloque))
  (Variables|/Game/Blueprints/FB/BP_SaveGameSystem.BP_SaveGameSystem_C|SetTournoi3Debloque _sauvegarde (Variables|FurnitureBattle|GetTournoi3Debloque))
  (|AsyncSaveGametoSlot _sauvegarde (Variables|FurnitureBattle|GetSaveName)))

(event Custom|AcheteUnMeuble
  (params (MeubleIndex :type Integer))
  ;[1 0.5427 0.2033 0.5 36] Acheter un Meuble
  (Utilities|Array|SetArrayElem (Variables|FurnitureBattle|GetMeublesPossedes) MeubleIndex true true))

(event Custom|Continue
  (bind _returnvalue (SaveGame|DoesSaveGameExist (Variables|FurnitureBattle|GetSaveName)))
  (if _returnvalue
    (CallFunction|LoadGame)
    (Utilities|FlowControl|Delay 0.5)
    (Game|OpenLevel(byName) "None")))

(event Custom|OpenLevel
  (Game|OpenLevel(byObjectReference) "/Game/Maps/Level_Main.Level_Main"))

(fn InitTournament
  (bind _allpossibletrainers (Variables|FurnitureBattle|GetAllPossibleTrainers))
  (bind _outrownames (DataTable|GetDataTableRowNames "/Game/Blueprints/FB/Battle/Dresseurs_Données.Dresseurs_Données"))
  (for _array_element _outrownames
    (bind _returnvalue (Utilities|GetDataTableRow "/Game/Blueprints/FB/Battle/Dresseurs_Données.Dresseurs_Données" _array_element)
      (:then
        (if (Utilities|Enum|Equal(Enum) (Variables|FurnitureBattle|GetTournoiDifficulte) (Utilities|Struct|BreakStruct_TrainerData _returnvalue))
          (Utilities|Array|Add (Variables|FurnitureBattle|GetAllPossibleTrainers) _returnvalue)))))
  (while (> (Utilities|Array|Length _allpossibletrainers) 3)
    (Utilities|Array|RemoveItem _allpossibletrainers (.OutItem (Utilities|Array|Random _allpossibletrainers))))
  (return (Variables|FurnitureBattle|GetAllPossibleTrainers)))