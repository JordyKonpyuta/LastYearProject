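; Game Instance that holds and saves player progression: money, owned furniture, win/loss record and tournament unlocks.
; New Game, Continue and load events manage a single BP_SaveGameSystem slot.
; Tournament completion pays out by difficulty and wins, unlocks the next tier at three wins, then saves (async for unlocks, sync for the rest).
; InitTournament filters the trainer data table by difficulty and randomly trims it to three opponents.
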(event Custom|NewGame
  (bind _returnvalue (SaveGame|DoesSaveGameExist (Variables|Default|GetSaveName)))
  (if _returnvalue
    (SaveGame|DeleteGameinSlot (Variables|Default|GetSaveName)))
  (CallFunction|CreateSaveData)
  (Utilities|FlowControl|Delay 0.5)
  (Game|OpenLevel(byName) "None"))

(event Custom|SaveGame
  (bind _sauvegarde (Variables|Default|GetSauvegarde))
  ;[0.1314 0.9203 1 0.5 48] Sauvegarde
  (Variables|/Game/Blueprints/BP_SaveGameSystem.BP_SaveGameSystem_C|SetArgent _sauvegarde (Variables|Default|GetArgentActuel))
  (Variables|/Game/Blueprints/BP_SaveGameSystem.BP_SaveGameSystem_C|SetMeublesDeverouilles _sauvegarde (Variables|Default|GetMeublesPossedes))
  (Variables|/Game/Blueprints/BP_SaveGameSystem.BP_SaveGameSystem_C|SetVictoires _sauvegarde (Variables|Default|GetVictoires))
  (Variables|/Game/Blueprints/BP_SaveGameSystem.BP_SaveGameSystem_C|SetDefaites _sauvegarde (Variables|Default|GetDefaites))
  (SaveGame|SaveGametoSlot _sauvegarde (Variables|Default|GetSaveName)))

(event Custom|LoadGame
  ;[1 0.7309 0 0.5 48] Load Save Data
  (bind _returnvalue (SaveGame|LoadGamefromSlot (Variables|Default|GetSaveName)))
  (bind _asbp_save_game_system (Utilities|Casting|CastToBP_SaveGameSystem _returnvalue))
  (bind _output_get (Variables|Default|SetSauvegarde _asbp_save_game_system))
  (Variables|Default|SetArgentActuel (Variables|/Game/Blueprints/BP_SaveGameSystem.BP_SaveGameSystem_C|GetArgent _output_get))
  (Variables|Default|SetMeublesPossedes (Variables|/Game/Blueprints/BP_SaveGameSystem.BP_SaveGameSystem_C|GetMeublesDeverouilles _output_get))
  (Variables|Default|SetVictoires (Variables|/Game/Blueprints/BP_SaveGameSystem.BP_SaveGameSystem_C|GetVictoires _output_get))
  (Variables|Default|SetDefaites (Variables|/Game/Blueprints/BP_SaveGameSystem.BP_SaveGameSystem_C|GetDefaites _output_get))
  (Variables|Default|SetTournoi2Debloque (Variables|/Game/Blueprints/BP_SaveGameSystem.BP_SaveGameSystem_C|GetTournoi2Debloque _output_get))
  (Variables|Default|SetTournoi3Debloque (Variables|/Game/Blueprints/BP_SaveGameSystem.BP_SaveGameSystem_C|GetTournoi3Debloque _output_get)))

(event Custom|Create%20Save%20Data
  ;[0.01548 0.15 0 0.5 36] Create Save Data
  (bind _returnvalue (SaveGame|CreateSaveGameObject "/Game/Blueprints/BP_SaveGameSystem.BP_SaveGameSystem_C"))
  (SaveGame|SaveGametoSlot _returnvalue (Variables|Default|GetSaveName))
  (Variables|Default|SetSauvegarde _returnvalue)
  (CallFunction|SaveGame))

(event Custom|TournoiTermine
  (params (NombreDeVictoires :type Integer))
  ;[0.6198 0.1355 0.4813 0.5 36] Completer un Tournoi
  (Variables|Default|SetGainArgent (Math|Float|Truncate (* (Utilities|Select :Index (Variables|Default|GetTournoiDifficulte) :NewEnumerator0 200 :NewEnumerator1 300 :NewEnumerator2 400) (Utilities|Select :Index NombreDeVictoires :Option%200 0.25 :Option%201 0.5 :Option%202 0.75 :Option%203 1.0))))
  (if (>= NombreDeVictoires 3)
    (Math|Integer|IncrementInt (Variables|Default|GetVictoires)
      (:%20%20
        (switch Utilities|FlowControl|Switch|SwitchonEnum_TournamentClass (Variables|Default|GetTournoiDifficulte)
          (:NewEnumerator0
            (Variables|Default|SetTournoi2Debloque true))
          (:NewEnumerator1
            (Variables|Default|SetTournoi3Debloque true))
          (:NewEnumerator2
            _))))
    (else
      (Math|Integer|IncrementInt (Variables|Default|GetDefaites)
        (:%20%20
          _))))
  (CallFunction|SauvegardeTournois)
  (Variables|Default|SetArgentActuel (+ (Variables|Default|GetArgentActuel) (Variables|Default|GetGainArgent)))
  (CallFunction|SaveGame))

(event Custom|SauvegardeTournois
  (bind _sauvegarde (Variables|Default|GetSauvegarde))
  ;[0 0.1703 1 0.5 30] Sauvegarde Spécifique - Tournois
  (Variables|/Game/Blueprints/BP_SaveGameSystem.BP_SaveGameSystem_C|SetTournoi2Debloque _sauvegarde (Variables|Default|GetTournoi2Debloque))
  (Variables|/Game/Blueprints/BP_SaveGameSystem.BP_SaveGameSystem_C|SetTournoi3Debloque _sauvegarde (Variables|Default|GetTournoi3Debloque))
  (|AsyncSaveGametoSlot _sauvegarde (Variables|Default|GetSaveName)))

(event Custom|AcheteUnMeuble
  (params (MeubleIndex :type Integer))
  ;[1 0.5427 0.2033 0.5 36] Acheter un Meuble
  (Utilities|Array|SetArrayElem (Variables|Default|GetMeublesPossedes) MeubleIndex true true))

(event Custom|Continue
  (bind _returnvalue (SaveGame|DoesSaveGameExist (Variables|Default|GetSaveName)))
  (if _returnvalue
    (CallFunction|LoadGame)
    (Utilities|FlowControl|Delay 0.5)
    (Game|OpenLevel(byName) "None")))

(event Custom|OpenLevel
  (Game|OpenLevel(byObjectReference) "/Game/Maps/Level_Main.Level_Main"))

(fn InitTournament
  (bind _allpossibletrainers (Variables|Default|GetAllPossibleTrainers))
  (bind _outrownames (DataTable|GetDataTableRowNames "/Game/Blueprints/Battle/Dresseurs_Données.Dresseurs_Données"))
  (for _array_element _outrownames
    (bind _returnvalue (Utilities|GetDataTableRow "/Game/Blueprints/Battle/Dresseurs_Données.Dresseurs_Données" _array_element)
      (:then
        (if (Utilities|Enum|Equal(Enum) (Variables|Default|GetTournoiDifficulte) (Utilities|Struct|BreakStruct_TrainerData _returnvalue))
          (Utilities|Array|Add (Variables|Default|GetAllPossibleTrainers) _returnvalue)))))
  (while (> (Utilities|Array|Length _allpossibletrainers) 3)
    (Utilities|Array|RemoveItem _allpossibletrainers (.OutItem (Utilities|Array|Random _allpossibletrainers))))
  (return (Variables|Default|GetAllPossibleTrainers)))