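; Spline object actor that moves a configurable static mesh along its spline, starting at BeginPlay.
; BeginPlay assigns ObjectMesh, then MoveObject plays a timeline with its rate set to the inverse of TimeToComplete.
; Each update maps the timeline track to distance along the spline and applies the local location and rotation there, with a 90-degree negative yaw offset.
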(event Custom|MoveObject
  (bind _spline (Variables|Default|GetSpline))
  (Components|Timeline|SetPlayRate (Variables|Default|GetT_Move) (/ 1.0 (Variables|Default|GetTimeToComplete)))
  (bind _newtrack_0 (Timeline|T_Move Play)
    (:Update
      (Transformation|SetRelativeLocationAndRotation (Variables|Default|GetStaticMesh) (Spline|GetLocationatDistanceAlongSpline _spline (Math|Float|Lerp 0.0 (Spline|GetSplineLength _spline) _newtrack_0) "Local") (Math|Rotator|MakeRotator (.roll (Spline|GetRotationatDistanceAlongSpline _spline (Math|Float|Lerp 0.0 (Spline|GetSplineLength _spline) _newtrack_0) "Local")) (.pitch (Spline|GetRotationatDistanceAlongSpline _spline (Math|Float|Lerp 0.0 (Spline|GetSplineLength _spline) _newtrack_0) "Local")) (- (.yaw (Spline|GetRotationatDistanceAlongSpline _spline (Math|Float|Lerp 0.0 (Spline|GetSplineLength _spline) _newtrack_0) "Local")) 9e+01)) false false))))

(event EventBeginPlay
  (Components|StaticMesh|SetStaticMesh (Variables|Default|GetStaticMesh) (Variables|Default|GetObjectMesh))
  (CallFunction|MoveObject))

(fn ConstructionScript)