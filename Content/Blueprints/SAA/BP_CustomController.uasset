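; BP_CustomController is a controller that opens the main menu and picks a random set of active instructions when play begins.
; InitInstructions fills ActiveInstructions by repeatedly drawing from a fixed list of ten enum values with AddUnique until it holds three distinct entries.
; BeginPlay runs that selection, then creates WBP_MainMenu and adds it to the viewport.
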(event Custom|InitInstructions
  (while (!= (Utilities|Array|Length (Variables|Default|GetActiveInstructions)) 3)
    (Utilities|Array|AddUnique (Variables|Default|GetActiveInstructions) (.OutItem (Utilities|Array|Random (Utilities|Array|MakeArray "NewEnumerator0" "NewEnumerator1" "NewEnumerator3" "NewEnumerator5" "NewEnumerator4" "NewEnumerator6" "NewEnumerator7" "NewEnumerator9" "NewEnumerator10" "NewEnumerator11"))))))

(event EventBeginPlay
  (CallFunction|InitInstructions)
  (bind _returnvalue (UserInterface|CreateWidget "/Game/Blueprints/SAA/WBP_MainMenu.WBP_MainMenu_C"))
  (UserInterface|Viewport|AddtoViewport _returnvalue 0))

(fn ConstructionScript)