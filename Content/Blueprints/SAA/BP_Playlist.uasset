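; BP_Playlist is a music player that steps through a list of tracks and drives a bar-style audio visualizer.
; Each track pairs with a Constant-Q analysis asset, sampled at the playback position to scale UI images vertically per band.
; A looping one-second timer counts elapsed time, letting playback resume after a pause and advancing to the next track when the current one ends.
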(event Custom|SetSoundToPlay
  (Variables|Default|SetSoundToPlay (Utilities|Array|Get(acopy) (Variables|Default|GetMusics) (Variables|Default|GetIndex)))
  (Variables|Default|SetDuration (Variables|/Script/Engine.SoundBase|GetDuration (Variables|Default|GetSoundToPlay)))
  (Audio|Components|Audio|SetSound (Variables|Default|GetAudio) (Variables|Default|GetSoundToPlay))
  (Variables|Default|SetConstant_Ref (Utilities|Array|Get(acopy) (Variables|Default|GetConstants) (Variables|Default|GetIndex))))

(event Custom|PauseSound
  (Audio|Components|Audio|Stop (Variables|Default|GetAudio))
  (Utilities|Time|PauseTimerbyHandle (Variables|Default|GetTimerHandle)))

(event Custom|PlaySound
  (Utilities|Time|UnpauseTimerbyHandle (Variables|Default|GetTimerHandle))
  (Audio|Components|Audio|Play (Variables|Default|GetAudio) (Variables|Default|GetElapsedTime))
  (bind _returnvalue (Utilities|Time|SetTimerbyEvent (delegate Custom|SetElapsedTime) 1.0 true))
  (Variables|Default|SetTimerHandle _returnvalue))

(event Custom|SetElapsedTime
  (if (< (Variables|Default|GetElapsedTime) (Variables|/Script/Engine.SoundBase|GetDuration (Variables|Default|GetSoundToPlay)))
    (Math|Float|IncrementFloat (Variables|Default|GetElapsedTime))
    (else
      (Variables|Default|SetElapsedTime 0.0)
      (Utilities|FlowControl|Delay 0.2)
      (Math|Integer|IncrementInt (Variables|Default|GetIndex)
        (:%20%20
          (CallFunction|SetSoundtoPlay)
          (CallFunction|PlaySound))))))

(event Custom|PlaybackChange
  (params (PlayingSoundWave :type Sound%20Wave%20Object%20Reference) (PlaybackPercent :type Float%20%28single-precision%29))
  (for (_array_element _array_index) (Class|ConstantQNRT|GetNormalizedChannelConstantQatTime (Variables|Default|GetConstant_Ref) (* PlaybackPercent (Variables|Default|GetDuration)))
    (Utilities|IsValid (Utilities|Array|Get(acopy) (Variables|Default|GetImages) _array_index)
      (:Is%20Valid
        (Variables|/Script/UMG.Widget|SetRenderTransform (Utilities|Array|Get(acopy) (Variables|Default|GetImages) _array_index) (Utilities|Struct|MakeWidgetTransform "(X=0.000000,Y=0.000000)" (Math|Vector2D|MakeVector2D 1.0 (* _array_element 3.0)) "(X=0.000000,Y=0.000000)" 0.0))))))

(event EventBeginPlay
  (CallFunction|SetSoundtoPlay)
  (EventDispatchers|BindEventtoOnAudioPlaybackPercent (Variables|Default|GetAudio) (delegate Custom|PlaybackChange)))

(fn ConstructionScript)