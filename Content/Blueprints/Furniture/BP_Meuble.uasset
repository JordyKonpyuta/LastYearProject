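; Furniture combatant actor, initialized from a data struct with name, health, attacks and speed, its mesh matched by name against the Meubles_Données table.
; AttaqueGenerale cycles two attacks in a set order, and additive percentage modifiers scale attack power and speed.
; Damage, heal and buff events drive the damage widget, Niagara effects and sounds, with death reported to the game mode before destruction.
; Timelines animate attack lunges and buff spins.
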(event Custom|CustomBeginPlay
  (params (Fourniture_BaseData :type Struct%20Furniture%20Data%20Structure%20%28by%20ref%29))
  (bind (_nom _description _icone _viemax _attaques _vitesse) (Utilities|Struct|BreakStruct_FurnitureData Fourniture_BaseData))
  ;[1 0.4633 0.2617 0.5 72] Begin Play
  (Variables|Default|SetNom _nom)
  (bind _output_get (Variables|Stats|SetVieMax _viemax))
  (Variables|Stats|SetVieActuelle _output_get)
  (Variables|Default|SetAttaques _attaques)
  (Variables|Stats|SetVitesse _vitesse)
  (bind _outrownames (DataTable|GetDataTableRowNames "/Game/Blueprints/Furniture/Meubles_Données.Meubles_Données"))
  (for (_array_element _array_index) _outrownames
    (bind _returnvalue (Utilities|GetDataTableRow "/Game/Blueprints/Furniture/Meubles_Données.Meubles_Données" _array_element)
      (:then
        (if (Utilities|Enum|Equal(Enum) (Variables|Default|GetNom) (.Nom (Utilities|Struct|BreakStruct_FurnitureData _returnvalue)))
          (Components|StaticMesh|SetStaticMesh (Variables|Default|GetStaticMesh) (Utilities|Select :Index _array_index :Option%200 "/Game/Assets/Meshes/poubelle.poubelle" :Option%201 "/Game/Assets/Meshes/lampe__1_.lampe__1_" :Option%202 "/Game/Assets/Meshes/arrosoir__1_.arrosoir__1_" :Option%203 "/Game/Assets/Meshes/ordinateur__1_.ordinateur__1_" :Option%204 "/Game/Assets/Meshes/commode.commode" :Option%205 "/Game/Assets/Meshes/chaise.chaise" :Option%206 "/Game/Assets/Meshes/Mesh_Adhesif.Mesh_Adhesif" :Option%207 "/Game/Assets/Meshes/four.four")))))))

(event Custom|DispDamage
  (params (Integer :type Integer))
  ;[0.15 0.15 0.15 0.5] All Widgets
  (bind _aswbp_damage (Utilities|Casting|CastToWBP_Damage (UserInterface|GetWidget (Variables|Default|GetDamageWidget))))
  (Default|DisplayDamage _aswbp_damage Integer))

(event Custom|Changement%20-%20Vitesse
  (params (BuffQuantity :type Integer))
  (bind _returnvalue (> BuffQuantity 0))
  ;[0.15 0.15 0.15 0.5] Various Effects
  (Utilities|Array|Add (Variables|Buffs|GetMulti_VitesseValues) (/ (Math|Conversions|ToFloat(Integer) BuffQuantity) 1e+02))
  (CallFunction|DispBuff _returnvalue false)
  (Niagara|SpawnSystematLocation (select _returnvalue "/Game/FX/NS_Buff.NS_Buff" "/Game/FX/NS_Debuff.NS_Debuff") (Transformation|GetActorLocation))
  (Audio|PlaySound2D "/Game/Assets/Sound/SFX/SC_Arrosage.SC_Arrosage" 1.0 1.0 0.0 0 0))

(event Custom|Changement%20-%20Attaque
  (params (BuffQuantity :type Integer))
  (bind _returnvalue (> BuffQuantity 0))
  ;[0.15 0.15 0.15 0.5] Various Effects
  (Utilities|Array|Add (Variables|Buffs|GetMulti_AttaqueValues) (/ (Math|Conversions|ToFloat(Integer) BuffQuantity) 1e+02))
  (CallFunction|DispBuff _returnvalue true)
  (Niagara|SpawnSystematLocation (select _returnvalue "/Game/FX/NS_Buff.NS_Buff" "/Game/FX/NS_Debuff.NS_Debuff") (Transformation|GetActorLocation))
  (Audio|PlaySound2D "/Game/Assets/Sound/SFX/SC_Flash.SC_Flash" 1.0 1.0 0.0 0 0))

(event Custom|DispHeal
  (params (Integer :type Integer))
  ;[0.15 0.15 0.15 0.5] All Widgets
  (bind _aswbp_damage (Utilities|Casting|CastToWBP_Damage (UserInterface|GetWidget (Variables|Default|GetDamageWidget))))
  (Default|DisplayHeal _aswbp_damage Integer))

(event Custom|TakeDamage
  (params (DamageValue :type Integer))
  ;[0.15 0.15 0.15 0.5] Various Effects
  (CallFunction|DispDamage DamageValue)
  (bind _output_get (Variables|Stats|SetVieActuelle (Math|Integer|SelectInt 0 (- (Variables|Stats|GetVieActuelle) DamageValue) (< (- (Variables|Stats|GetVieActuelle) DamageValue) 0))))
  (Niagara|SpawnSystematLocation "/Game/FX/NS_Hit.NS_Hit" (Transformation|GetActorLocation))
  (Audio|PlaySound2D "/Game/Assets/Sound/SFX/SC_Hit.SC_Hit" 1.0 1.0 0.0 0 0)
  (if (<= _output_get 0)
    (bind _gamemoderef (Variables|Default|GetGamemodeRef)
      (:then
        (Default|DeadMeuble _gamemoderef self)
        (Utilities|FlowControl|Delay 0.2)
        (Actor|DestroyActor))
      (:else))))

(event Custom|Heal
  (params (HealValue :type Integer))
  ;[0.15 0.15 0.15 0.5] Various Effects
  (CallFunction|DispHeal HealValue)
  (Variables|Stats|SetVieActuelle (Math|Integer|SelectInt (Variables|Stats|GetVieMax) (+ HealValue (Variables|Stats|GetVieActuelle)) (> (+ HealValue (Variables|Stats|GetVieActuelle)) (Variables|Stats|GetVieMax))))
  (Niagara|SpawnSystematLocation "/Game/FX/NS_Heal.NS_Heal" (Transformation|GetActorLocation))
  (Audio|PlaySound2D "/Game/Assets/Sound/SFX/SC_Adhesif.SC_Adhesif" 1.0 1.0 0.0 0 0))

(event Custom|Play%20Animation
  (bind _newtrack_0 (Timeline|Attack PlayFromStart)
    (:Update
      _)
    (:Finished
      _))
  (Transformation|SetRelativeLocation (Variables|Default|GetStaticMesh) (Math|Vector|Lerp(Vector) "0, 0, 0" (* (Class|KismetMathLibrary|VectorForward) 45.0) _newtrack_0) false false))

(event Custom|DispBuff
  (params (Buff :type Boolean) (Attaque :type Boolean))
  ;[0.15 0.15 0.15 0.5] All Widgets
  (bind _aswbp_damage (Utilities|Casting|CastToWBP_Damage (UserInterface|GetWidget (Variables|Default|GetDamageWidget))))
  (Default|DisplayBuff _aswbp_damage Buff Attaque))

(event Custom|PlayBuffAnim
  (Variables|Default|SetRotRef (Transformation|GetActorRotation))
  (bind _newtrack_0 (Timeline|Timeline PlayFromStart)
    (:Update
      (Transformation|SetActorRotation (Math|Rotator|Lerp(Rotator) (Variables|Default|GetRotRef) (Math|Rotator|MakeRotator (.Roll (Math|Rotator|BreakRotator (Variables|Default|GetRotRef))) (.Pitch (Math|Rotator|BreakRotator (Variables|Default|GetRotRef))) (+ (.Yaw (Math|Rotator|BreakRotator (Variables|Default|GetRotRef))) 3.6e+02)) _newtrack_0)))
    (:Finished
      (Transformation|SetActorRotation (Variables|Default|GetRotRef)))))

(fn ConstructionScript)

(fn Attaque1
  (bind _attaques (Variables|Default|GetAttaques))
  (bind _output (Utilities|Array|Get(acopy) _attaques))
  (bind (_cible _effetdelattaque _valeurprincipale _valeursecondaire) (Utilities|Struct|BreakStruct_AttackData _output))
  (return _cible _effetdelattaque (CallFunction|NouvellePuissance _valeurprincipale) _valeursecondaire))

(fn Attaque2
  (bind _attaques (Variables|Default|GetAttaques))
  (bind _output (Utilities|Array|Get(acopy) _attaques 1))
  (bind (_cible _effetdelattaque _valeurprincipale _valeursecondaire) (Utilities|Struct|BreakStruct_AttackData _output))
  (return _cible _effetdelattaque (Math|Integer|SelectInt (CallFunction|NouvellePuissance _valeurprincipale) _valeurprincipale (Utilities|IsItBuffable _effetdelattaque)) _valeursecondaire))

(fn AttaqueGenerale
  (bind (_cible _effet_de_l_attaque _valeur_principale _valeur_secondaire) (CallFunction|Attaque1))
  (bind (_cible_2 _effet_de_l_attaque_2 _valeur_principale_2 _valeur_secondaire_2) (CallFunction|Attaque2))
  (switch int (Utilities|Array|Get(acopy) (Variables|AttaqueSelection|GetOrdreDesAttaques) (Variables|AttaqueSelection|GetPositionDansLaFileDesAttaques))
    (:Default
      (Variables|AttaqueSelection|SetPositionDansLaFileDesAttaques 0))
    (:0
      (Variables|AttaqueSelection|SetPositionDansLaFileDesAttaques (Math|Integer|SelectInt 0 (+ (Variables|AttaqueSelection|GetPositionDansLaFileDesAttaques) 1) (== (+ (Variables|AttaqueSelection|GetPositionDansLaFileDesAttaques) 1) (Utilities|Array|Length (Variables|AttaqueSelection|GetOrdreDesAttaques))))))
    (:1
      (Variables|AttaqueSelection|SetPositionDansLaFileDesAttaques (Math|Integer|SelectInt 0 (+ (Variables|AttaqueSelection|GetPositionDansLaFileDesAttaques) 1) (== (+ (Variables|AttaqueSelection|GetPositionDansLaFileDesAttaques) 1) (Utilities|Array|Length (Variables|AttaqueSelection|GetOrdreDesAttaques)))))
      (return _cible_2 _effet_de_l_attaque_2 _valeur_principale_2 _valeur_secondaire_2)))
  (return _cible _effet_de_l_attaque _valeur_principale _valeur_secondaire))

(fn NouvellePuissance
  (params (DegatsBase :type Integer))
  (bind _multi_attaquevalues (Variables|Buffs|GetMulti_AttaqueValues))
  (if (Utilities|Array|IsEmpty _multi_attaquevalues)
    (return DegatsBase)
    (else
      (LocalVariables|SetBuffActuel 1.0)
      (for _array_element _multi_attaquevalues
        (LocalVariables|SetBuffActuel (+ _array_element (LocalVariables|GetBuffActuel))))
      (return (Math|Integer|SelectInt 1 (Math|Float|Truncate (* (LocalVariables|GetBuffActuel) DegatsBase)) (< (Math|Float|Truncate (* (LocalVariables|GetBuffActuel) DegatsBase)) 1))))))

(fn GetTrueSpeed
  (LocalVariables|SetTotalSpeedMulti 1.0)
  (for _array_element (Variables|Buffs|GetMulti_VitesseValues)
    (LocalVariables|SetTotalSpeedMulti (+ (LocalVariables|GetTotalSpeedMulti) _array_element)))
  (return (Math|Integer|SelectInt 0 (Math|Float|Truncate (* (Variables|Stats|GetVitesse) (LocalVariables|GetTotalSpeedMulti))) (< (Math|Float|Truncate (* (Variables|Stats|GetVitesse) (LocalVariables|GetTotalSpeedMulti))) 0))))